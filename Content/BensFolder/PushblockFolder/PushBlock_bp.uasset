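; Push block actor that the ThirdPersonCharacter can move, with trigger boxes meant to restrict pushing to the sides rather than diagonals.
; Entering either the Xbox or Ybox trigger turns on physics simulation on the Block, and leaving either turns it off.
; The construction script gives the Block a dynamic Push_Block_M material, coloured green when Target is set and red otherwise.
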(event OnComponentBeginOverlap(ybox)
  (params (OverlappedComponent :type Primitive%20Component%20Object%20Reference) (OtherActor :type Actor%20Object%20Reference) (OtherComp :type Primitive%20Component%20Object%20Reference) (OtherBodyIndex :type Integer) (bFromSweep :type Boolean) (SweepResult :type Hit%20Result%20Structure%20%28by%20ref%29))
  ;[1 1 1] Limits cube to be push from sides only not diagonaly
  (Utilities|Casting|CastToThirdPersonCharacter OtherActor)
  (Physics|SetSimulatePhysics (Variables|Default|GetBlock) true))

(event OnComponentEndOverlap(ybox)
  (params (OverlappedComponent :type Primitive%20Component%20Object%20Reference) (OtherActor :type Actor%20Object%20Reference) (OtherComp :type Primitive%20Component%20Object%20Reference) (OtherBodyIndex :type Integer))
  ;[1 1 1] Limits cube to be push from sides only not diagonaly
  (Utilities|Casting|CastToThirdPersonCharacter OtherActor)
  (Physics|SetSimulatePhysics (Variables|Default|GetBlock) false))

(event OnComponentBeginOverlap(xbox)
  (params (OverlappedComponent :type Primitive%20Component%20Object%20Reference) (OtherActor :type Actor%20Object%20Reference) (OtherComp :type Primitive%20Component%20Object%20Reference) (OtherBodyIndex :type Integer) (bFromSweep :type Boolean) (SweepResult :type Hit%20Result%20Structure%20%28by%20ref%29))
  ;[1 1 1] Limits cube to be push from sides only not diagonaly
  (Utilities|Casting|CastToThirdPersonCharacter OtherActor)
  (Physics|SetSimulatePhysics (Variables|Default|GetBlock) true))

(event OnComponentEndOverlap(xbox)
  (params (OverlappedComponent :type Primitive%20Component%20Object%20Reference) (OtherActor :type Actor%20Object%20Reference) (OtherComp :type Primitive%20Component%20Object%20Reference) (OtherBodyIndex :type Integer))
  ;[1 1 1] Limits cube to be push from sides only not diagonaly
  (Utilities|Casting|CastToThirdPersonCharacter OtherActor)
  (Physics|SetSimulatePhysics (Variables|Default|GetBlock) false))

(event Collision|EventActorBeginOverlap
  (params (OtherActor :type Actor%20Object%20Reference)))

(event EventTick
  (params (DeltaSeconds :type Float%20%28single-precision%29)))

(fn ConstructionScript
  (bind _block (Variables|Default|GetBlock))
  (bind _returnvalue (Rendering|Material|CreateDynamicMaterialInstance _block 0 "/Game/BensFolder/PushblockFolder/Push_Block_M.Push_Block_M" "None" :!class /Script/Engine.PrimitiveComponent))
  (Rendering|Material|SetMaterial _block 0 _returnvalue)
  (if (Variables|Default|GetTarget?)
    (Rendering|Material|SetVectorParameterValue _returnvalue "Colour" "(R=0.014836,G=1.000000,B=0.000000,A=1.000000)" :!class /Script/Engine.MaterialInstanceDynamic)
    (else
      (Rendering|Material|SetVectorParameterValue _returnvalue "Colour" "(R=1.000000,G=0.000000,B=0.009549,A=1.000000)" :!class /Script/Engine.MaterialInstanceDynamic))))